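; A10 actor for a precision air strike that flies a spline track, fires at the player character's strike location, then destroys itself.
; A timeline scaled by Duration moves it along TrackRef's spline.
; A delayed effects sequence plays smoke, sounds and muzzle Niagara while a looping timer spawns BP_Projectile tracers toward random points in a box.
; A debug-drawn box trace at the strike location supplies that box's origin; damage is not implemented.
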(event `self.ReceiveBeginPlay`
  (bind _percisionstrikelocation (`self.PercisionStrikeLocation`))
  (`self.StartPercisionAirStrike`)
  (bind _asbp_character (cast `/Game/Blueprints/Characters/BP_Character` (`GameplayStatics.GetPlayerPawn` 0)))
  (set `self.PercisionStrikeLocation` (`/Game/Blueprints/Characters/BP_Character.PercisionStrikeLocation` _asbp_character))
  (`self.PlayEffects`)
  ;[1 1 1] Creating a BoxTrace so we can deal damage to actors within that box (I didn't add dealing damage functionality)
  (bind _outhit (`KismetSystemLibrary.BoxTraceSingle` :`Start` _percisionstrikelocation :`End` _percisionstrikelocation :`HalfSize` (`self.BoxExtent`) :`Orientation` (`KismetMathLibrary.Conv_VectorToRotator` (`SceneComponent.GetForwardVector` (`self.A10_StaticMesh`))) :`TraceChannel` "TraceTypeQuery1" :`DrawDebugType` "Persistent"))
  (set `self.HitResults` _outhit))

(event `StartPercisionAirStrike`
  (bind _a10splinepath (`/Game/Blueprints/Actors/BP_Track.A10SplinePath` (`self.TrackRef`)))
  (bind _returnvalue (`KismetMathLibrary.Lerp` 0.0 (`SplineComponent.GetSplineLength` _a10splinepath) (`self.Alpha`)))
  ;[1 1 1] Attaching the A10 to the tracks and make it move through the spline
  (`TimelineComponent.SetPlayRate` (`self.TimeLine_A10Mover`) (/ 1.0 (`self.Duration`)))
  (bind (_direction _alpha) (`Timeline|TimeLine_A10Mover`)
    (:`Update`
      (set `self.Alpha` _alpha)
      (`self.K2_SetActorLocationAndRotation` (`SplineComponent.GetLocationAtDistanceAlongSpline` _a10splinepath _returnvalue "World") (`SplineComponent.GetRotationAtDistanceAlongSpline` _a10splinepath _returnvalue "World")))
    (:`Finished`
      (`self.K2_DestroyActor`))))

(event `PlayEffects`
  ;[1 1 1] Playing the A10 effects
  (`GameplayStatics.SpawnEmitterAttached` "/Game/Assets/Effects/P_SmokeTrail.P_SmokeTrail" (`self.SmokeTrailRightWing`))
  (`GameplayStatics.SpawnEmitterAttached` "/Game/Assets/Effects/P_SmokeTrail.P_SmokeTrail" (`self.SmokeTrailLeftWing`))
  (`GameplayStatics.SpawnSoundAttached` "/Game/Assets/SoundEffects/A10/A_PercisionA10_Cue.A_PercisionA10_Cue" (`self.A10_StaticMesh`) "None" (0.0 0.0 0.0) (struct) "KeepRelativeOffset" false 1.0 1.0 0.0 null null)
  (`KismetSystemLibrary.Delay` 1.0)
  (bind _returnvalue (`GameplayStatics.SpawnSoundAttached` "/Game/Assets/SoundEffects/A10/A_FireFirstSound_Cue.A_FireFirstSound_Cue" (`self.A10_StaticMesh`) "None" (0.0 0.0 0.0) (struct) "KeepRelativeOffset" false 1.0 1.0 0.0 null null))
  (bind _returnvalue_2 (`NiagaraFunctionLibrary.SpawnSystemAttached` "/Game/Assets/Effects/NiagaraEffects/N_Muzzle_System.N_Muzzle_System" (`self.ProjectileSpawnPoint`) "None" (0.0 0.0 0.0) (struct) "KeepRelativeOffset" true))
  (bind _returnvalue_3 (`KismetSystemLibrary.K2_SetTimer` null "SpawnProjectiles" 0.1 true))
  (`KismetSystemLibrary.Delay` (`SoundBase.Duration` (`AudioComponent.Sound` _returnvalue)))
  (`GameplayStatics.SpawnSoundAttached` "/Game/Assets/SoundEffects/A10/A_FireSecondSound_Cue.A_FireSecondSound_Cue" (`self.A10_StaticMesh`) "None" (0.0 0.0 0.0) (struct) "KeepRelativeOffset" false 1.0 1.0 0.0 null null)
  (`SceneComponent.K2_DetachFromComponent` _returnvalue_2 "KeepRelative" "KeepRelative" "KeepRelative" true)
  (`KismetSystemLibrary.Delay` 0.7)
  (`KismetSystemLibrary.K2_ClearAndInvalidateTimerHandle` _returnvalue_3))

(event `SpawnProjectiles`
  ;[1 1 1] Spawning Bullet Traces
  (bind _returnvalue (`|SpawnActorFromClass` "/Game/Blueprints/Actors/BP_Projectile.BP_Projectile_C" (`SceneComponent.K2_GetComponentToWorld` (`self.ProjectileSpawnPoint`)) "AlwaysSpawn" "OverrideRootScale" null null))
  (set `/Game/Blueprints/Actors/BP_Projectile.InterpolationDuration` 0.5 _returnvalue)
  (set `/Game/Blueprints/Actors/BP_Projectile.Target` (`self.GetRandomPointInBox`) _returnvalue)
  (`/Game/Blueprints/Actors/BP_Projectile.SpawnParticle` _returnvalue))

(fn `GetRandomPointInBox`
  (returns (PointLocation :type "Vector Structure"))
  (return (`KismetMathLibrary.RandomPointInBoundingBox` (`.Location` (`GameplayStatics.BreakHitResult` (`self.HitResults`))) (`self.BoxExtent`))))

(fn `UserConstructionScript`)